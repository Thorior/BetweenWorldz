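; Moving platform that slides its static mesh back and forth along its local X axis in an endless loop from BeginPlay.
; Raise plays one timeline forward and Fall plays a second in reverse, each calling the other on finish.
; Both scale their movement track into a relative X location, so motion is horizontal despite the event names.
; The Delay variable is only assigned to itself and never pauses the cycle.
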(event Custom|Fall
  (bind _movementtrack (Timeline|Timeline_2 ReverseFromEnd)
    (:Update
      (Transformation|SetRelativeLocation (Variables|Default|GetStaticMesh) (Math|Vector|MakeVector (* _movementtrack 1e+03) 0.0 0.0) false false))
    (:Finished
      (CallFunction|Raise))))

(event Custom|Raise
  (bind _movementtrack (Timeline|Timeline_0 PlayFromStart)
    (:Update
      (Transformation|SetRelativeLocation (Variables|Default|GetStaticMesh) (Math|Vector|MakeVector (* _movementtrack 1e+03) 0.0 0.0) false false))
    (:Finished
      (CallFunction|Fall))))

(event EventBeginPlay
  (Variables|Default|SetDelay (Variables|Default|GetDelay))
  (CallFunction|Raise))

(fn ConstructionScript)