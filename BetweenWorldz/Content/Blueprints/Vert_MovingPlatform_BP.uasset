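; A vertical moving platform that rises and falls in an endless loop from the start of play.
; Raise plays one timeline forward and Fall plays a second in reverse from its end, each triggering the other when finished.
; Both scale their float track to set the StaticMesh's relative Z location, moving only the mesh component.
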(event Custom|Fall
  (bind _risefltrack (Timeline|Timeline_1 ReverseFromEnd)
    (:Update
      (Transformation|SetRelativeLocation (Variables|Default|GetStaticMesh) (Math|Vector|MakeVector 0.0 0.0 (* _risefltrack 1e+03)) false false))
    (:Finished
      (CallFunction|Raise))))

(event Custom|Raise
  (bind _risefltrack (Timeline|Timeline_0 PlayFromStart)
    (:Update
      (Transformation|SetRelativeLocation (Variables|Default|GetStaticMesh) (Math|Vector|MakeVector 0.0 0.0 (* _risefltrack 1e+03)) false false))
    (:Finished
      (CallFunction|Fall))))

(event EventBeginPlay
  (Variables|Default|SetDelay (Variables|Default|GetDelay))
  (CallFunction|Raise))

(fn ConstructionScript)