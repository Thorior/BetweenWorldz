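; BossMob2_BP is a boss enemy that loses health to player projectiles and loads Level1 when defeated.
; On BeginPlay it passes itself to the BossHealthBar widget from its widget component and refreshes it.
; Each overlap with a player projectile subtracts a fixed amount of health and updates the bar.
; When health drops below zero, it sets IsDead, destroys itself and opens the level.
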(event EventBeginPlay
  (bind _asboss_health_bar (Utilities|Casting|CastToBossHealthBar (UserInterface|GetUserWidgetObject (Variables|Default|GetBossHealthBar))))
  (bind _output_get (Variables|Default|SetAs%20Boss%20Health%20Bar _asboss_health_bar))
  (Variables|/Game/Blueprints/Enemies/Enemy_UI/BossHealthBar.BossHealthBar_C|SetBoss _output_get self)
  (Default|UpdateHealth _asboss_health_bar))

(event Collision|EventActorBeginOverlap
  (params (OtherActor :type Actor%20Object%20Reference))
  (Utilities|Casting|CastToPlayerCharacterProjectile_BP OtherActor)
  (Variables|Default|SetHealth (- (Variables|Default|GetHealth) 0.1))
  (Default|UpdateHealth (Variables|Default|GetAs%20Boss%20Health%20Bar))
  (if (< (Variables|Default|GetHealth) 0.0)
    (Variables|Default|SetIsDead true)
    (Actor|DestroyActor)
    (Game|OpenLevel(byName) "Level1")))

(fn ConstructionScript)