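; ObjectiveCollect_BP is a spinning objective pickup that raises vertical platforms when overlapped.
; On BeginPlay it caches every TriggeredPlatformVert_BP in the level, and three index variables select platforms from that array.
; Any actor overlap plays a pull sound, sets Activated and calls Raise on those three platforms, then destroys the pickup.
; Tick applies a fixed local rotation each frame, without delta-time scaling.
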(event EventBeginPlay
  (bind _outactors (Actor|GetAllActorsOfClass "/Game/Blueprints/TriggeredPlatformVert_BP.TriggeredPlatformVert_BP_C"))
  (Variables|Default|SetTriggeredPlatform _outactors))

(event Collision|EventActorBeginOverlap
  (params (OtherActor :type Actor%20Object%20Reference))
  (bind _platform_index_2 (Variables|Default|GetPlatform_Index#2))
  (bind _triggeredplatform (Variables|Default|GetTriggeredPlatform))
  (bind _triggeredplatform_2 (Variables|Default|GetTriggeredPlatform))
  (bind _triggeredplatform_3 (Variables|Default|GetTriggeredPlatform))
  (bind _platform_index_3 (Variables|Default|GetPlatform_Index#3))
  (bind _platform_index_ (Variables|Default|GetPlatform_Index#))
  (bind _output (Utilities|Array|Get(acopy) _triggeredplatform _platform_index_3))
  (bind _output_2 (Utilities|Array|Get(acopy) _triggeredplatform_2 _platform_index_))
  (bind _output_3 (Utilities|Array|Get(acopy) _triggeredplatform_3 _platform_index_2))
  (Audio|PlaySoundatLocation "/Engine/VREditor/Sounds/UI/Laser_Pull.Laser_Pull" (Transformation|GetActorLocation (Components|GetOwner (Variables|Default|GetDefaultSceneRoot))) "0, 0, 0" 1.5 1.0 0.0 0 0 0)
  (CallFunction|CallRaise _output_2 _output_2)
  (CallFunction|CallRaise _output_3 _output_3)
  (CallFunction|CallRaise _output _output)
  (Actor|DestroyActor))

(event EventTick
  (params (DeltaSeconds :type Float%20%28single-precision%29))
  (Transformation|AddLocalRotation (Variables|Default|GetDefaultSceneRoot) "0.500000,2.000000,1.500000" false false))

(fn ConstructionScript)

(fn CallRaise
  (params (self2 :type Triggered%20Platform%20Vert%20BP%20Object%20Reference) (self3 :type Triggered%20Platform%20Vert%20BP%20Object%20Reference))
  (Variables|/Game/Blueprints/TriggeredPlatformVert_BP.TriggeredPlatformVert_BP_C|SetActivated self2 true)
  (Default|Raise self3))